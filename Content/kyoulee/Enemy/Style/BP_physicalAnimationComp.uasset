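; Actor component that gives BP_Player or BP_Enemy_Base owners physics-driven hit and death reactions through a PhysicalAnimationComponent created at BeginPlay.
; HitReaction applies a profile, simulates bodies from spine_01 down the chain if alive, and always adds an impulse at the hit bone.
; Tick decays a short timer as physics blend weight, then stops simulation and itself.
; DeadReaction stops Tick and simulates from the pelvis with a death profile.
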(event Custom|TogglePhysicalAnimation
  ;[1 1 1] 흐느적 거리게 만들기
  (Class|SkeletalMeshComponent|SetAllBodiesBelowSimulatePhysics (Variables|Default|GetMesh) (Utilities|Name|MakeLiteralName "spine_01") true false)
  ;[1 1 1] physical 강도 조절 2가지방법
  ;;[1 1 1] 좀더 직관적인 1 ~ 0 사이로 조절한다
  (Class|SkeletalMeshComponent|SetAllBodiesBelowPhysicsBlendWeight (Variables|Default|GetMesh) (Utilities|Name|MakeLiteralName "spine_01") 0.5 false true))

(event Custom|DeadReaction
  ;[1 1 1] Dead Reaction
  (Components|Tick|SetComponentTickEnabled false)
  (Class|PhysicalAnimationComponent|ApplyPhysicalAnimationProfileBelow (Variables|Default|GetPhysicalAnimationComp) "selvis" "Dead" false false)
  (Class|SkeletalMeshComponent|SetAllBodiesBelowSimulatePhysics (Variables|Default|GetMesh) (Utilities|Name|MakeLiteralName "pelvis") true true))

(event Custom|HitReaction
  (params (Hit :type Hit%20Result%20Structure%20%28by%20ref%29) (Dead :type Boolean) (SkeletalMesh :type Skeletal%20Mesh%20Component%20Object%20Reference))
  (bind (_bblockinghit _binitialoverlap _time _distance _location _impactpoint _normal _impactnormal _physmat _hitactor _hitcomponent _hitbonename _bonename _hititem _elementindex _faceindex _tracestart _traceend) (Collision|BreakHitResult Hit))
  ;[1 1 1] 아파하기
  (if (not Dead)
    (Components|Tick|SetComponentTickEnabled false)
    (Variables|Default|SetHitReactionTimeRemaining (Math|Float|Min(Float) (+ (Variables|Default|GetHitReactionTimeRemaining) 1.0) 0.5))
    ;;[1 1 1] 물리 ㄱ용하기
    (Class|PhysicalAnimationComponent|ApplyPhysicalAnimationProfileBelow (Variables|Default|GetPhysicalAnimationComp) "spine_01" "Storg" false false)
    (Class|SkeletalMeshComponent|SetAllBodiesBelowSimulatePhysics (Variables|Default|GetMesh) (Utilities|Name|MakeLiteralName "spine_01") true true)
    ;;[1 1 1] 맞은 본 찾기
    (Components|Tick|SetComponentTickEnabled true))
  (Physics|AddImpulse (Variables|Default|GetMesh) (* (Math|Vector|Normalize (- _traceend _tracestart)) 5e+03) _hitbonename true))

(event EventBeginPlay
  (bind _returnvalue (Components|GetOwner))
  (bind _returnvalue_2 (Game|AddComponentbyClass (Components|GetOwner) "/Script/Engine.PhysicalAnimationComponent"))
  (bind _output_get (Variables|Default|SetPhysicalAnimationComp _returnvalue_2))
  (Utilities|FlowControl|Sequence
    (:then_0
      (bind _asbp_player (Utilities|Casting|CastToBP_Player _returnvalue))
      (Variables|Default|SetMesh (Variables|/Script/Engine.Character|GetMesh _asbp_player))
      (Class|PhysicalAnimationComponent|SetSkeletalMeshComponent _output_get (Variables|/Script/Engine.Character|GetMesh _asbp_player)))
    (:then_1
      (bind _asbp_enemy_base (Utilities|Casting|CastToBP_Enemy_Base _returnvalue))
      (Variables|Default|SetMesh (Variables|/Script/Engine.Character|GetMesh _asbp_enemy_base))
      (Class|PhysicalAnimationComponent|SetSkeletalMeshComponent _output_get (Variables|/Script/Engine.Character|GetMesh _asbp_enemy_base)))))

(event EventTick
  (params (DeltaSeconds :type Float%20%28single-precision%29))
  ;[1 1 1] 아파하기 점점 축소
  (Variables|Default|SetHitReactionTimeRemaining (- (Math|Interpolation|FInterpTo (Variables|Default|GetHitReactionTimeRemaining) 0.0 0.0 1.0) (* DeltaSeconds 1.0)))
  (if (<= (Variables|Default|GetHitReactionTimeRemaining) 0.0)
    (Variables|Default|SetHitReactionTimeRemaining 0.0)
    (Class|SkeletalMeshComponent|SetAllBodiesBelowSimulatePhysics (Variables|Default|GetMesh) (Utilities|Name|MakeLiteralName "spine_01") false true)
    (Components|Tick|SetComponentTickEnabled false)
    (else
      (Class|SkeletalMeshComponent|SetAllBodiesBelowPhysicsBlendWeight (Variables|Default|GetMesh) (Utilities|Name|MakeLiteralName "spine_01") (Math|Float|Min(Float) (Variables|Default|GetHitReactionTimeRemaining) 1.0) false true))))