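; BP_DoorDouble is a double door actor whose two leaves swing open and closed in opposite directions.
; OpenDoor, CloseDoor and ToggleDoor only set the IsOpen flag, which Tick reads to step CurrRotation toward MaxRotation or back toward zero at Speed.
; Tick applies that angle as mirrored relative yaw on DoorLeft and DoorRight.
; BeginPlay honors an initially open state and enables player input, though no input events are bound here.
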(event Custom|ToggleDoor
  (if (Variables|Default|GetIsOpen)
    (CallFunction|CloseDoor)
    (else
      (CallFunction|OpenDoor))))

(event Custom|CloseDoor
  (Variables|Default|SetIsOpen false))

(event Custom|OpenDoor
  (Variables|Default|SetIsOpen true))

(event EventTick
  (params (DeltaSeconds :type Float%20%28single-precision%29))
  (if (Variables|Default|GetIsOpen)
    ;[1 1 1] 회전 열림
    (if (< (Variables|Default|GetCurrRotation) (Variables|Default|GetMaxRotation))
      (bind _output_get (Variables|Default|SetCurrRotation (+ (Variables|Default|GetCurrRotation) (* DeltaSeconds (Variables|Default|GetSpeed)))))
      (Transformation|SetRelativeRotation (Variables|Default|GetDoorLeft) (Math|Rotator|MakeRotator 0.0 0.0 _output_get) false false)
      (Transformation|SetRelativeRotation (Variables|Default|GetDoorRight) (Math|Rotator|MakeRotator 0.0 0.0 (* _output_get -1.0)) false false))
    (else
      ;[1 1 1] Comment
      (if (>= (Variables|Default|GetCurrRotation) 0.0)
        (bind _output_get_2 (Variables|Default|SetCurrRotation (- (Variables|Default|GetCurrRotation) (* DeltaSeconds (Variables|Default|GetSpeed)))))
        (Transformation|SetRelativeRotation (Variables|Default|GetDoorLeft) (Math|Rotator|MakeRotator 0.0 0.0 _output_get_2) false false)
        (Transformation|SetRelativeRotation (Variables|Default|GetDoorRight) (Math|Rotator|MakeRotator 0.0 0.0 (* _output_get_2 -1.0)) false false)))))

(event Collision|EventActorBeginOverlap
  (params (OtherActor :type Actor%20Object%20Reference)))

(event EventBeginPlay
  (Utilities|FlowControl|Sequence
    (:then_0
      (if (Variables|Default|GetIsOpen)
        (CallFunction|OpenDoor)))
    (:then_1
      (Input|EnableInput (Game|GetPlayerController 0)))))

(fn ConstructionScript)