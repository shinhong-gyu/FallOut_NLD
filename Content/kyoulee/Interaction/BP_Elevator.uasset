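; Elevator actor with four sliding door panels that open after a floor call and close again.
; CallElevator only steps the Floor counter to the called floor, using in-loop Delays flagged as possibly broken, then sets IsOpen.
; Tick slides left and right panels oppositely along local Y through MoveYLocation, tracking travel in DoorCurront.
; Opening plays a Delay-gated 2D sound; once fully open, a Delay clears IsOpen to close the doors.
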(event Custom|CallElevator
  (params (CallFloor :type Integer))
  ;[1 1 1] call elevator delay maybe not working
  (if (> CallFloor (Variables|Default|GetFloor))
    (for _index (range (Variables|Default|GetFloor) CallFloor)
      (Variables|Default|SetFloor (+ (Variables|Default|GetFloor) 1))
      (Utilities|FlowControl|Delay 1.0))
    (Variables|Default|SetIsOpen true)
    (else
      (for _index_2 (range CallFloor (Variables|Default|GetFloor))
        (Variables|Default|SetFloor (- (Variables|Default|GetFloor) 1))
        (Utilities|FlowControl|Delay 1.0))
      (Variables|Default|SetIsOpen true))))

(event EventBeginPlay)

(event Collision|EventActorBeginOverlap
  (params (OtherActor :type Actor%20Object%20Reference)))

(event EventTick
  (params (DeltaSeconds :type Float%20%28single-precision%29))
  (bind _speed (Variables|Default|GetSpeed))
  (bind _speed_2 (Variables|Default|GetSpeed))
  (bind _returnvalue (* _speed_2 DeltaSeconds))
  (bind _returnvalue_2 (* _speed DeltaSeconds))
  (bind _returnvalue_3 (* _returnvalue -1.0))
  (bind _returnvalue_4 (* _returnvalue_2 -1.0))
  (if (Variables|Default|GetIsOpen)
    ;[1 1 1] Elevator Opening
    (if (< (Variables|Default|GetDoorCurront) (Variables|Default|GetDoorTransForm))
      (CallFunction|MoveYLocation (Variables|Default|GetLeftDoor1) _returnvalue_2)
      (CallFunction|MoveYLocation (Variables|Default|GetLeftDoor2) _returnvalue_2)
      (CallFunction|MoveYLocation (Variables|Default|GetRightDoor1) _returnvalue_4)
      (CallFunction|MoveYLocation (Variables|Default|GetRightDoor2) _returnvalue_4)
      (Variables|Default|SetDoorCurront (+ (Variables|Default|GetDoorCurront) _returnvalue_2))
      (if (not (Variables|Default|GetSoundPlay))
        (Variables|Default|SetSoundPlay true)
        (Audio|PlaySound2D "/Game/kyoulee/Sounds/Assets/SD_SlidingDoorBarn.SD_SlidingDoorBarn" 1.0 1.0 0.0 0 0)
        (Utilities|FlowControl|Delay 8.0)
        (Variables|Default|SetSoundPlay false))
      (else
        (Utilities|FlowControl|Delay 3.0)
        (Variables|Default|SetIsOpen false)))
    (else
      ;[1 1 1] Close Door
      (if (> (Variables|Default|GetDoorCurront) 0.0)
        (CallFunction|MoveYLocation (Variables|Default|GetLeftDoor1) _returnvalue_3)
        (CallFunction|MoveYLocation (Variables|Default|GetLeftDoor2) _returnvalue_3)
        (CallFunction|MoveYLocation (Variables|Default|GetRightDoor1) _returnvalue)
        (CallFunction|MoveYLocation (Variables|Default|GetRightDoor2) _returnvalue)
        (Variables|Default|SetDoorCurront (- (Variables|Default|GetDoorCurront) _returnvalue))))))

(fn ConstructionScript)

(fn MoveYLocation
  (params (Target :type Scene%20Component%20Object%20Reference) (Move :type Float%20%28double-precision%29))
  (bind _returnvalue (Transformation|GetRelativeTransform Target))
  (Transformation|SetRelativeLocation Target (Math|Vector|MakeVector (.x (.location _returnvalue)) (+ Move (.y (.location _returnvalue))) (.z (.location _returnvalue))) false false))